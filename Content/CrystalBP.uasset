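; CrystalBP is a crystal that explodes when Hugo comes near after enough enemies are defeated.
; Tick polls the player's distance and checks EnemiesDefeated in MyGame, then plays the blast effect and sound and destroys itself with attached actors.
; Below the kill threshold, a DoOnce shows the Kill5 widget.
; While out of range, every tick removes all Kill5 widgets and resets the DoOnce.
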(event `self.ReceiveTick`
  (params (DeltaSeconds :type "Float (single-precision)"))
  (bind _ashugo (cast `/Game/CaveAssets/Characters/Hugo` (`GameplayStatics.GetPlayerCharacter` 0)))
  (if (< (`self.GetDistanceTo` _ashugo) 600.0)
    (bind _asmy_game (cast `/Game/CaveAssets/Characters/MyGame` (`GameplayStatics.GetGameMode`)))
    (if (>= (`/Game/CaveAssets/Characters/MyGame.EnemiesDefeated` _asmy_game) 3)
      (`GameplayStatics.SpawnEmitterAtLocation` "/Game/InfinityBladeEffects/Effects/FX_Ability/Defense/P_EnergyBlast_Impact.P_EnergyBlast_Impact" (`self.K2_GetActorLocation` self) (struct) (4.0 4.0 4.0))
      (`GameplayStatics.PlaySound2D` "/Game/StarterContent/Audio/Explosion02.Explosion02")
      (`self.K2_DestroyActor` (`self.GetAttachedActors`))
      (`self.K2_DestroyActor`)
      (else
        (`/Engine/EditorBlueprintResources/StandardMacros.DoOnce` false :!label _label
          (:`Completed`
            (bind _returnvalue (`|CreateWidget` "/Game/Kill5.Kill5_C"))
            (`UserWidget.AddToViewport` _returnvalue 0)))))
    (else
      (bind _foundwidgets (`WidgetBlueprintLibrary.GetAllWidgetsOfClass` "/Game/Kill5.Kill5_C" false))
      (`Widget.RemoveFromParent` _foundwidgets)
      (goto _label :!via `Reset`))))

(fn `UserConstructionScript`)